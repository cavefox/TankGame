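; BP_Tank is a controllable tank that wires player input to its aiming, movement and camera components.
; BeginPlay gives TankAiming the barrel and turret meshes, TankMovement the two tracks, and sets the tank as the health bar widget's owner.
; Input orbits the camera via an azimuth node and spring arm, fires through TankAiming and passes drive intent to TankMovement.
; Tick yaws the health bar to face against the player camera's view direction.
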(event `self.ReceiveBeginPlay`
  (`TankAimingComponent.Initialise` (`self.TankAiming`) (`self.TankBarrelMesh`) (`self.TurretMesh`))
  (`TankMovementComponent.Initialise` (`self.TankMovement`) (`self.TankLeftTrack`) (`self.TankRightTrack`))
  (bind _ashealth_bar (cast `/Game/Widgets/HealthBar` (`WidgetComponent.GetUserWidgetObject` (`self.Health Bar`))))
  (set `/Game/Widgets/HealthBar.Owner` self _ashealth_bar))

(event `self.ReceiveTick`
  (params (DeltaSeconds :type "Float (single-precision)"))
  (bind (_returnvalue_roll _returnvalue_pitch _returnvalue_yaw) (`KismetMathLibrary.BreakRotator` (`KismetMathLibrary.MakeRotFromX` (* (`SceneComponent.GetForwardVector` (`PlayerCameraManager.TransformComponent` (`PlayerController.PlayerCameraManager` (`GameplayStatics.GetPlayerController` 0)))) -1.0))))
  (`SceneComponent.K2_SetWorldRotation` (`self.Health Bar`) (`KismetMathLibrary.MakeRotator` 0.0 0.0 _returnvalue_yaw) false false))

(event `InputAxis|AimAzimuth`
  (params (AxisValue :type "Float (single-precision)"))
  ;[1 1 1] Aiming And Fire
  (`SceneComponent.K2_AddLocalRotation` (`self.CamAzimuthNode`) (`KismetMathLibrary.MakeRotator` 0.0 0.0 (* AxisValue (`GameplayStatics.GetWorldDeltaSeconds`) 100.0)) false false))

(event `InputAxis|AimElevation`
  (params (AxisValue :type "Float (single-precision)"))
  ;[1 1 1] Aiming And Fire
  (`SceneComponent.K2_AddLocalRotation` (`self.SpringArm`) (`KismetMathLibrary.MakeRotator` 0.0 (* AxisValue (`GameplayStatics.GetWorldDeltaSeconds`) 100.0)) false false))

(event `InputAction|Fire`
  (params (Key :type "Key Structure" :default "AnyKey"))
  ;[1 1 1] Aiming And Fire
  (:`Pressed`
    (`TankAimingComponent.Fire` (`self.TankAiming`))))

(event `InputAxis|MoveForward`
  (params (AxisValue :type "Float (single-precision)"))
  ;[1 1 1] Input for Tank Movement
  (`TankMovementComponent.IntendToMoveForward` (`self.TankMovement`) AxisValue))

(event `InputAxis|TurnRight`
  (params (AxisValue :type "Float (single-precision)"))
  ;[1 1 1] Input for Tank Movement
  (`TankMovementComponent.IntendToTurnRight` (`self.TankMovement`) AxisValue))

(fn `UserConstructionScript`)